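; BP_PositionResetZone is a trigger zone that returns lab props to their respawn points when they enter it.
; On overlap it casts the actor to a flask, container or electricity element, in that order, and ignores anything else.
; It turns off physics simulation on the prop's mesh, moves the actor to its own stored respawn position, then re-enables physics.
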(event `self.Trigger.OnComponentBeginOverlap`
  (params (OverlappedComponent :type "PrimitiveComponent Object Reference") (OtherActor :type "Actor Object Reference") (OtherComp :type "PrimitiveComponent Object Reference") (OtherBodyIndex :type Integer) (bFromSweep :type Boolean) (SweepResult :type "HitResult Structure (by ref)"))
  (bind _asbp_flask_parent (cast `/Game/EducationVR/Blueprints/Chemistry/BP_FlaskParent` OtherActor)
    (:`then`
      (bind _output_get (set `self.LastObjectFlask` _asbp_flask_parent))
      (`PrimitiveComponent.SetSimulatePhysics` (`/Game/EducationVR/Blueprints/Chemistry/BP_FlaskParent.StaticMesh` _output_get) false)
      (`self.K2_SetActorLocation` _asbp_flask_parent (`/Game/EducationVR/Blueprints/Chemistry/BP_FlaskParent.RespawnLocation` (`self.LastObjectFlask`)) false false)
      (`PrimitiveComponent.SetSimulatePhysics` (`/Game/EducationVR/Blueprints/Chemistry/BP_FlaskParent.StaticMesh` (`self.LastObjectFlask`)) true))
    (:`CastFailed`
      (bind _asbp_container_parent (cast `/Game/EducationVR/Blueprints/Chemistry/BP_ContainerParent` OtherActor)
        (:`then`
          (bind _output_get_2 (set `self.LastObjectContainer` _asbp_container_parent))
          (`PrimitiveComponent.SetSimulatePhysics` (`/Game/EducationVR/Blueprints/Chemistry/BP_ContainerParent.StaticMesh` _output_get_2) false)
          (`self.K2_SetActorLocation` _asbp_container_parent (`/Game/EducationVR/Blueprints/Chemistry/BP_ContainerParent.RespawnPosition` (`self.LastObjectContainer`)) false false)
          (`PrimitiveComponent.SetSimulatePhysics` (`/Game/EducationVR/Blueprints/Chemistry/BP_ContainerParent.StaticMesh` (`self.LastObjectContainer`)) true))
        (:`CastFailed`
          (bind _asbp_electricity_element (cast `/Game/EducationVR/Blueprints/Electricity/BP_ElectricityElement` OtherActor))
          (bind _output_get_3 (set `self.LastObjectElectricityElement` _asbp_electricity_element))
          (`PrimitiveComponent.SetSimulatePhysics` (`/Game/EducationVR/Blueprints/Electricity/BP_ElectricityElement.StaticMesh` _output_get_3) false)
          (`self.K2_SetActorLocation` _asbp_electricity_element (`/Game/EducationVR/Blueprints/Electricity/BP_ElectricityElement.RespawnLocation` (`self.LastObjectElectricityElement`)) false false)
          (`PrimitiveComponent.SetSimulatePhysics` (`/Game/EducationVR/Blueprints/Electricity/BP_ElectricityElement.StaticMesh` (`self.LastObjectElectricityElement`)) true))))))

(fn `UserConstructionScript`)