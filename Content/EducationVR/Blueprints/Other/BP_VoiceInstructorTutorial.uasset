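; BP_VoiceInstructorTutorial is a voice instructor for the VR education tutorial that plays spoken audio clips.
; On BeginPlay it finds the BP_Controller, plays the first clip after a short delay, then after a longer timed delay makes the controller's widget visible.
; PlayAudio stops any clip already playing, swaps in the requested sound from an array by index and plays it from the start.
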(event `self.ReceiveBeginPlay`
  (bind _returnvalue (`GameplayStatics.GetActorOfClass` "/Game/EducationVR/Blueprints/UI/BP_Controller.BP_Controller_C"))
  (`KismetSystemLibrary.Delay` 2.0)
  (`self.PlayAudio` 0)
  (`KismetSystemLibrary.Delay` 28.0)
  (`SceneComponent.SetVisibility` (`/Game/EducationVR/Blueprints/UI/BP_Controller.Widget` _returnvalue) true false))

(fn `PlayAudio`
  (params (AudioIndex :type Integer))
  (bind _audio (`self.Audio`))
  (if (`AudioComponent.IsPlaying` (`self.Audio`))
    (`AudioComponent.Stop` _audio))
  (`AudioComponent.SetSound` _audio (`|GetArrayItem` (`self.SoundArr`) AudioIndex))
  (`AudioComponent.Play` (`self.Audio`) 0.0))

(fn `UserConstructionScript`)