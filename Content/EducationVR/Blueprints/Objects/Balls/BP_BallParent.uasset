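; Base VR physics ball for an educational throwing demo, showing ball properties and throw forces.
; While held it logs velocities; on release it applies their average, updates the throw, gravity and air resistance readouts, and triggers a scene capture.
; Gravity and air resistance arrows follow the ball after a throw.
; Floor hits play speed-scaled bounce sounds, while repeated low-bounce hits respawn the ball and hide the arrows.
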(event `self.ReceiveBeginPlay`
  (bind _returnvalue (`GameplayStatics.GetActorOfClass` "/Game/EducationVR/Blueprints/Objects/BP_CaptureCam.BP_CaptureCam_C"))
  (set `self.CaptureCam` _returnvalue))

(event `self.GrabComponent.OnGrabbed`
  (set `self.bIsHeld` true)
  (set `self.MeshMass` (`PrimitiveComponent.GetMass` (`self.Mesh`)))
  (`self.DisplayBallStats`))

(event `self.GrabComponent.OnDropped`
  (`SceneComponent.SetVisibility` (`self.GravityArrow`) true false)
  (`SceneComponent.SetVisibility` (`self.AirResistanceArrow`) true false)
  (`PrimitiveComponent.SetPhysicsLinearVelocity` (`self.Mesh`) (`KismetMathLibrary.GetVectorArrayAverage` (`self.VelLog`)) false "None")
  (set `self.bIsHeld` false)
  (set `self.InitialVelocity` (`SceneComponent.GetComponentVelocity` (`self.Mesh`)))
  (`self.DisplayThrowStats`)
  (`SceneCaptureComponent2D.CaptureScene` (`/Game/EducationVR/Blueprints/Objects/BP_CaptureCam.SceneCaptureComponent2D` (`self.CaptureCam`))))

(event `self.ReceiveTick`
  (params (DeltaSeconds :type "Float (single-precision)"))
  (bind (_returnvalue_x _returnvalue_y _returnvalue_z) (`KismetMathLibrary.BreakVector` (`SceneComponent.K2_GetComponentLocation` (`self.Mesh`))))
  (bind (_returnvalue_x_2 _returnvalue_y_2 _returnvalue_z_2) (`KismetMathLibrary.BreakVector` (`SceneComponent.K2_GetComponentLocation` (`self.Mesh`))))
  (`SceneComponent.K2_SetWorldLocationAndRotation` (`self.GravityArrow`) (`KismetMathLibrary.MakeVector` _returnvalue_x_2 _returnvalue_y_2 (+ _returnvalue_z_2 50.0)) (struct :`Pitch` -90.0) false false)
  (bind _returnvalue (`PrimitiveComponent.GetPhysicsLinearVelocity` (`self.Mesh`) "None"))
  (`SceneComponent.K2_SetWorldLocationAndRotation` (`self.AirResistanceArrow`) (`KismetMathLibrary.MakeVector` _returnvalue_x _returnvalue_y _returnvalue_z) (`KismetMathLibrary.Conv_VectorToRotator` (`self.AirResistanceArrowDir`)) false false)
  (if (`self.bIsHeld`)
    (bind _returnvalue_2 (`PrimitiveComponent.GetPhysicsLinearVelocity` (`self.Mesh`) "None"))
    (`KismetArrayLibrary.Array_Set` (`self.VelLog`) (`self.VelLogIndex`) _returnvalue_2)
    (if (> (`self.VelLogIndex`) (`KismetArrayLibrary.Array_Length` (`self.VelLog`)))
      (set `self.VelLogIndex` 0)
      (else
        (`/Engine/EditorBlueprintResources/StandardMacros.IncrementInt` (`self.VelLogIndex`))))))

(event `self.ReceiveHit`
  (params (MyComp :type "PrimitiveComponent Object Reference") (Other :type "Actor Object Reference") (OtherComp :type "PrimitiveComponent Object Reference") (bSelfMoved :type Boolean) (HitLocation :type "Vector Structure") (HitNormal :type "Vector Structure") (NormalImpulse :type "Vector Structure") (Hit :type "HitResult Structure (by ref)"))
  (bind _mesh (`self.Mesh`))
  (bind _mesh_2 (`self.Mesh`))
  (bind (_returnvalue_x _returnvalue_y _returnvalue_z) (`KismetMathLibrary.BreakVector` (`SceneComponent.GetComponentVelocity` _mesh_2)))
  (bind _bisfloor (`self.CheckIfBouncableSurface` Other))
  (if _bisfloor
    (if (> _returnvalue_z 30.0)
      (`GameplayStatics.PlaySoundAtLocation` (`AudioComponent.Sound` (`self.Audio`)) HitLocation (struct) (`KismetMathLibrary.MapRangeClamped` (`KismetMathLibrary.VSize` (`SceneComponent.GetComponentVelocity` _mesh_2)) 0.0 1000.0 0.25 1.0) 1.0 0.0 null null null null)
      (elif (< (`self.ResetCounter`) 150)
        (`/Engine/EditorBlueprintResources/StandardMacros.IncrementInt` (`self.ResetCounter`))
        (else
          (`self.K2_SetActorLocation` (`self.BallRespawnPoint`))
          (`PrimitiveComponent.SetSimulatePhysics` _mesh false)
          (`PrimitiveComponent.SetSimulatePhysics` _mesh true)
          (set `self.ResetCounter` 0)
          (`SceneComponent.SetVisibility` (`self.GravityArrow`) false false)
          (`SceneComponent.SetVisibility` (`self.AirResistanceArrow`) false false))))))

(fn `CheckIfBouncableSurface`
  (params (HitActor :type "Actor Object Reference"))
  (returns (bIsFloor :type Boolean))
  (if (`self.ActorHasTag` HitActor "Floor")
    (return true)
    (else
      (return false))))

(fn `DisplayBallStats`
  (bind _returnvalue_x (`KismetMathLibrary.BreakVector` (`SceneComponent.K2_GetComponentScale` (`self.Mesh`))))
  (bind _returnvalue (`GameplayStatics.GetActorOfClass` "/Game/EducationVR/Blueprints/Objects/Displays/BP_BallInfoDisplay.BP_BallInfoDisplay_C"))
  (bind _aswbp_ball_info_display_panel (cast `/Game/EducationVR/UI/BallsModule/WBP_BallInfoDisplayPanel` (`WidgetComponent.GetWidget` (`/Game/EducationVR/Blueprints/Objects/Displays/BP_BallInfoDisplay.Widget` _returnvalue))))
  (set `self.BallInfoDisplayWidget` _aswbp_ball_info_display_panel)
  (set `TextBlock.Text` (`self.BallType`) (`/Game/EducationVR/UI/BallsModule/WBP_BallInfoDisplayPanel.BallTypeText` (`self.BallInfoDisplayWidget`)))
  (set `TextBlock.Text` (`self.BallMaterialType`) (`/Game/EducationVR/UI/BallsModule/WBP_BallInfoDisplayPanel.BallMaterialText` (`self.BallInfoDisplayWidget`)))
  (set `TextBlock.Text` (`|FormatText` "{diameter} cm" (* _returnvalue_x 100.0)) (`/Game/EducationVR/UI/BallsModule/WBP_BallInfoDisplayPanel.BallDiameterText` (`self.BallInfoDisplayWidget`)))
  (set `TextBlock.Text` (`|FormatText` "{mass} kg" (`self.MeshMass`)) (`/Game/EducationVR/UI/BallsModule/WBP_BallInfoDisplayPanel.BallMassText` (`self.BallInfoDisplayWidget`))))

(fn `DisplayThrowStats`
  (bind _returnvalue_x (`KismetMathLibrary.BreakVector` (`SceneComponent.K2_GetComponentScale` (`self.Mesh`))))
  (bind _returnvalue (`GameplayStatics.GetActorOfClass` "/Game/EducationVR/Blueprints/Objects/Displays/BP_ThrowInfoDisplay.BP_ThrowInfoDisplay_C"))
  (bind _aswbp_throw_info_display_panel (cast `/Game/EducationVR/UI/BallsModule/WBP_ThrowInfoDisplayPanel` (`WidgetComponent.GetWidget` (`/Game/EducationVR/Blueprints/Objects/Displays/BP_ThrowInfoDisplay.Widget` _returnvalue))))
  (set `self.ThrowInfoDisplayWidget` _aswbp_throw_info_display_panel)
  (set `TextBlock.Text` (`|FormatText` "{throwForce}N" (/ (* (`self.MeshMass`) (/ (`KismetMathLibrary.VSize` (`self.InitialVelocity`)) 100.0)) 0.2)) (`/Game/EducationVR/UI/BallsModule/WBP_ThrowInfoDisplayPanel.ThrowForceText` (`self.ThrowInfoDisplayWidget`)))
  (set `TextBlock.Text` (`|FormatText` "{gravity}N" (* (`self.MeshMass`) 9.81)) (`/Game/EducationVR/UI/BallsModule/WBP_ThrowInfoDisplayPanel.GravitationForceText` (`self.ThrowInfoDisplayWidget`)))
  (set `TextBlock.Text` (`|FormatText` "{air}N" (* (* (* (* 0.5 1.225) (* (/ (`KismetMathLibrary.VSize` (`self.InitialVelocity`)) 100.0) 2.0)) (`self.BallAirResistanceValue`)) (`KismetMathLibrary.MultiplyByPi` (* _returnvalue_x 2.0)))) (`/Game/EducationVR/UI/BallsModule/WBP_ThrowInfoDisplayPanel.AirResistanceForceText` (`self.ThrowInfoDisplayWidget`))))

(fn `UserConstructionScript`)