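; Base chemistry container for an educational VR lab that receives liquid from flasks and pours it out when tilted.
; A flask overlapping PourTrigger starts a looping timer that raises the fill level while that flask pours.
; DetermineFluidColor maps the first liquid ID, then one second-liquid mix, to data-table flow colors and hardcoded materials.
; Delay-throttled Tick checks tilt to drain the fluid and drive the flow effect and pouring sound.
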(event `self.PourTrigger.OnComponentBeginOverlap`
  (params (OverlappedComponent :type "PrimitiveComponent Object Reference") (OtherActor :type "Actor Object Reference") (OtherComp :type "PrimitiveComponent Object Reference") (OtherBodyIndex :type Integer) (bFromSweep :type Boolean) (SweepResult :type "HitResult Structure (by ref)"))
  (bind _asbp_flask_parent (cast `/Game/EducationVR/Blueprints/Chemistry/BP_FlaskParent` OtherActor))
  (set `self.Flask` _asbp_flask_parent)
  (`KismetSystemLibrary.K2_SetTimer` null "FillContainer" 0.1 true false 0.3))

(event `self.PourTrigger.OnComponentEndOverlap`
  (params (OverlappedComponent :type "PrimitiveComponent Object Reference") (OtherActor :type "Actor Object Reference") (OtherComp :type "PrimitiveComponent Object Reference") (OtherBodyIndex :type Integer))
  (cast `/Game/EducationVR/Blueprints/Chemistry/BP_FlaskParent` OtherActor)
  (set `self.Flask` null)
  (`KismetSystemLibrary.K2_ClearTimer` null "FillContainer"))

(event `self.ReceiveTick`
  (params (DeltaSeconds :type "Float (single-precision)"))
  (bind (_returnvalue_x _returnvalue_y _returnvalue_z) (`KismetMathLibrary.BreakVector` (`SceneComponent.GetUpVector` (`self.StaticMesh`))))
  (`KismetSystemLibrary.Delay` 0.1)
  (if (< _returnvalue_z (`self.RotationThreshold`))
    (if (`self.bIsLiquidInside`)
      (`ActorComponent.SetActive` (`self.Flow`) true false)
      (set `self.bIsPouring` true)
      (bind _output_get (set `self.FluidLevel` (`KismetMathLibrary.FClamp` (- (`self.FluidLevel`) 0.01))))
      (`NiagaraComponent.SetVariableFloat` (`self.Fluid`) "Fill" _output_get)
      (if (<= (`self.FluidLevel`) 0.0)
        (`ActorComponent.SetActive` (`self.Flow`) false false)
        (set `self.bIsPouring` false)
        (set `self.bIsFluidInside` false)
        (set `self.bAreTwoLiquidsInside` false)
        (set `self.bIsSoundPlaying` false)
        (`AudioComponent.Stop` (`self.Audio`))
        (elif (not (`self.bIsSoundPlaying`))
          (set `self.bIsSoundPlaying` true)
          (`AudioComponent.Play` (`self.Audio`) 0.0)
          (`KismetSystemLibrary.Delay` 3.8)
          (set `self.bIsSoundPlaying` false)))
      (else
        (`ActorComponent.SetActive` (`self.Flow`) false false :!label _label)
        (set `self.bIsPouring` false)
        (set `self.bIsSoundPlaying` false)
        (`AudioComponent.Stop` (`self.Audio`))))
    (else
      (goto _label))))

(fn `DetermineFluidColor`
  (params (FluidID :type Integer))
  (bind (_datatable _rowname) (break `DataTableRowHandle` (`|GetArrayItem` (`self.DTTest`) 15)))
  (bind (_datatable_2 _rowname_2) (break `DataTableRowHandle` (`|GetArrayItem` (`self.DTTest`))))
  (bind (_datatable_3 _rowname_3) (break `DataTableRowHandle` (`|GetArrayItem` (`self.DTTest`) 1)))
  (bind (_datatable_4 _rowname_4) (break `DataTableRowHandle` (`|GetArrayItem` (`self.DTTest`) 2)))
  (bind (_datatable_5 _rowname_5) (break `DataTableRowHandle` (`|GetArrayItem` (`self.DTTest`) 4)))
  (bind (_datatable_6 _rowname_6) (break `DataTableRowHandle` (`|GetArrayItem` (`self.DTTest`) 6)))
  (bind (_datatable_7 _rowname_7) (break `DataTableRowHandle` (`|GetArrayItem` (`self.DTTest`) 7)))
  (bind (_datatable_8 _rowname_8) (break `DataTableRowHandle` (`|GetArrayItem` (`self.DTTest`) 8)))
  (bind (_datatable_9 _rowname_9) (break `DataTableRowHandle` (`|GetArrayItem` (`self.DTTest`) 9)))
  (bind (_datatable_10 _rowname_10) (break `DataTableRowHandle` (`|GetArrayItem` (`self.DTTest`) 10)))
  (bind (_datatable_11 _rowname_11) (break `DataTableRowHandle` (`|GetArrayItem` (`self.DTTest`) 11)))
  (bind (_datatable_12 _rowname_12) (break `DataTableRowHandle` (`|GetArrayItem` (`self.DTTest`) 12)))
  (bind (_datatable_13 _rowname_13) (break `DataTableRowHandle` (`|GetArrayItem` (`self.DTTest`) 13)))
  (bind (_datatable_14 _rowname_14) (break `DataTableRowHandle` (`|GetArrayItem` (`self.DTTest`) 3)))
  (bind (_datatable_15 _rowname_15) (break `DataTableRowHandle` (`|GetArrayItem` (`self.DTTest`) 14)))
  (bind (_datatable_16 _rowname_16) (break `DataTableRowHandle` (`|GetArrayItem` (`self.DTTest`) 5)))
  (if (not (`self.bIsFluidInside`))
    (set `self.bIsFluidInside` true)
    (switch `int` FluidID
      (:`1`
        (bind _returnvalue (`|GetDataTableRow` _datatable_2 _rowname_2)
          (:`then`
            (bind _output_get (set `self.StartColor` (`.Color_5_710DF73E405FA430BE76E1955AAA3F73` (break `/Game/EducationVR/Data/S_FluidColors` _returnvalue))))
            (`NiagaraComponent.SetVariableLinearColor` (`self.Flow`) "Color" _output_get)
            (set `self.FluidInsideID` 1)
            (`NiagaraComponent.SetVariableMaterial` (`self.Fluid`) "Material" "/Game/LiquidMaterials_VFXPack/Materials/Liquids/MI_Liquid_01.MI_Liquid_01"))))
      (:`2`
        (bind _returnvalue_2 (`|GetDataTableRow` _datatable_3 _rowname_3)
          (:`then`
            (bind _output_get_2 (set `self.StartColor` (`.Color_5_710DF73E405FA430BE76E1955AAA3F73` (break `/Game/EducationVR/Data/S_FluidColors` _returnvalue_2))))
            (`NiagaraComponent.SetVariableLinearColor` (`self.Flow`) "Color" _output_get_2)
            (set `self.FluidInsideID` 2)
            (`NiagaraComponent.SetVariableMaterial` (`self.Fluid`) "Material" "/Game/LiquidMaterials_VFXPack/Materials/Liquids/MI_Liquid_02.MI_Liquid_02"))))
      (:`3`
        (bind _returnvalue_3 (`|GetDataTableRow` _datatable_4 _rowname_4)
          (:`then`
            (bind _output_get_3 (set `self.StartColor` (`.Color_5_710DF73E405FA430BE76E1955AAA3F73` (break `/Game/EducationVR/Data/S_FluidColors` _returnvalue_3))))
            (`NiagaraComponent.SetVariableLinearColor` (`self.Flow`) "Color" _output_get_3)
            (set `self.FluidInsideID` 3)
            (`NiagaraComponent.SetVariableMaterial` (`self.Fluid`) "Material" "/Game/LiquidMaterials_VFXPack/Materials/Liquids/MI_Liquid_03.MI_Liquid_03"))))
      (:`4`
        (bind _returnvalue_4 (`|GetDataTableRow` _datatable_14 _rowname_14)
          (:`then`
            (bind _output_get_4 (set `self.StartColor` (`.Color_5_710DF73E405FA430BE76E1955AAA3F73` (break `/Game/EducationVR/Data/S_FluidColors` _returnvalue_4))))
            (`NiagaraComponent.SetVariableLinearColor` (`self.Flow`) "Color" _output_get_4)
            (set `self.FluidInsideID` 4)
            (`NiagaraComponent.SetVariableMaterial` (`self.Fluid`) "Material" "/Game/LiquidMaterials_VFXPack/Materials/Liquids/MI_Liquid_04.MI_Liquid_04")))))
    (elif (and (== (`self.FluidInsideID`) 1) (not (`self.bAreTwoLiquidsInside`)))
      (switch `int` FluidID
        (:`1`
          (return))
        (:`2`
          (bind _returnvalue_5 (`|GetDataTableRow` _datatable_5 _rowname_5)
            (:`then`
              (`NiagaraComponent.SetVariableLinearColor` (`self.Flow`) "Color" (`.Color_5_710DF73E405FA430BE76E1955AAA3F73` (break `/Game/EducationVR/Data/S_FluidColors` _returnvalue_5)))
              (`NiagaraComponent.SetVariableMaterial` (`self.Fluid`) "Material" "/Game/LiquidMaterials_VFXPack/Materials/Liquids/MI_Liquid_Green.MI_Liquid_Green"))))
        (:`3`
          (bind _returnvalue_6 (`|GetDataTableRow` _datatable_16 _rowname_16)
            (:`then`
              (`NiagaraComponent.SetVariableLinearColor` (`self.Flow`) "Color" (`.Color_5_710DF73E405FA430BE76E1955AAA3F73` (break `/Game/EducationVR/Data/S_FluidColors` _returnvalue_6)))
              (`NiagaraComponent.SetVariableMaterial` (`self.Fluid`) "Material" "/Game/LiquidMaterials_VFXPack/Materials/Liquids/MI_Liquid_Brown.MI_Liquid_Brown"))))
        (:`4`
          (bind _returnvalue_7 (`|GetDataTableRow` _datatable_6 _rowname_6)
            (:`then`
              (`NiagaraComponent.SetVariableLinearColor` (`self.Flow`) "Color" (`.Color_5_710DF73E405FA430BE76E1955AAA3F73` (break `/Game/EducationVR/Data/S_FluidColors` _returnvalue_7)))
              (`NiagaraComponent.SetVariableMaterial` (`self.Fluid`) "Material" "/Game/LiquidMaterials_VFXPack/Materials/Liquids/MI_Liquid_Colorless_Brown.MI_Liquid_Colorless_Brown")))))
      (set `self.bAreTwoLiquidsInside` true)
      (elif (and (== (`self.FluidInsideID`) 2) (not (`self.bAreTwoLiquidsInside`)))
        (switch `int` FluidID
          (:`1`
            (bind _returnvalue_8 (`|GetDataTableRow` _datatable_7 _rowname_7)
              (:`then`
                (`NiagaraComponent.SetVariableLinearColor` (`self.Flow`) "Color" (`.Color_5_710DF73E405FA430BE76E1955AAA3F73` (break `/Game/EducationVR/Data/S_FluidColors` _returnvalue_8)))
                (`NiagaraComponent.SetVariableMaterial` (`self.Fluid`) "Material" "/Game/LiquidMaterials_VFXPack/Materials/Liquids/MI_Liquid_Green.MI_Liquid_Green"))))
          (:`2`
            (return))
          (:`3`
            (bind _returnvalue_9 (`|GetDataTableRow` _datatable_8 _rowname_8)
              (:`then`
                (`NiagaraComponent.SetVariableLinearColor` (`self.Flow`) "Color" (`.Color_5_710DF73E405FA430BE76E1955AAA3F73` (break `/Game/EducationVR/Data/S_FluidColors` _returnvalue_9)))
                (`NiagaraComponent.SetVariableMaterial` (`self.Fluid`) "Material" "/Game/LiquidMaterials_VFXPack/Materials/Liquids/MI_Liquid_Yellow.MI_Liquid_Yellow"))))
          (:`4`
            (bind _returnvalue_10 (`|GetDataTableRow` _datatable_9 _rowname_9)
              (:`then`
                (`NiagaraComponent.SetVariableLinearColor` (`self.Flow`) "Color" (`.Color_5_710DF73E405FA430BE76E1955AAA3F73` (break `/Game/EducationVR/Data/S_FluidColors` _returnvalue_10)))
                (`NiagaraComponent.SetVariableMaterial` (`self.Fluid`) "Material" "/Game/LiquidMaterials_VFXPack/Materials/Liquids/MI_Liquid_LightGreen_Brown.MI_Liquid_LightGreen_Brown")))))
        (set `self.bAreTwoLiquidsInside` true)
        (elif (and (== (`self.FluidInsideID`) 3) (not (`self.bAreTwoLiquidsInside`)))
          (switch `int` FluidID
            (:`1`
              (bind _returnvalue_11 (`|GetDataTableRow` _datatable_10 _rowname_10)
                (:`then`
                  (`NiagaraComponent.SetVariableLinearColor` (`self.Flow`) "Color" (`.Color_5_710DF73E405FA430BE76E1955AAA3F73` (break `/Game/EducationVR/Data/S_FluidColors` _returnvalue_11)))
                  (`NiagaraComponent.SetVariableMaterial` (`self.Fluid`) "Material" "/Game/LiquidMaterials_VFXPack/Materials/Liquids/MI_Liquid_Brown.MI_Liquid_Brown"))))
            (:`2`
              (bind _returnvalue_12 (`|GetDataTableRow` _datatable_11 _rowname_11)
                (:`then`
                  (`NiagaraComponent.SetVariableLinearColor` (`self.Flow`) "Color" (`.Color_5_710DF73E405FA430BE76E1955AAA3F73` (break `/Game/EducationVR/Data/S_FluidColors` _returnvalue_12)))
                  (`NiagaraComponent.SetVariableMaterial` (`self.Fluid`) "Material" "/Game/LiquidMaterials_VFXPack/Materials/Liquids/MI_Liquid_Yellow.MI_Liquid_Yellow"))))
            (:`3`
              (return))
            (:`4`
              (bind _returnvalue_13 (`|GetDataTableRow` _datatable_12 _rowname_12)
                (:`then`
                  (`NiagaraComponent.SetVariableLinearColor` (`self.Flow`) "Color" (`.Color_5_710DF73E405FA430BE76E1955AAA3F73` (break `/Game/EducationVR/Data/S_FluidColors` _returnvalue_13)))
                  (`NiagaraComponent.SetVariableMaterial` (`self.Fluid`) "Material" "/Game/LiquidMaterials_VFXPack/Materials/Liquids/MI_Liquid_Green.MI_Liquid_Green")))))
          (set `self.bAreTwoLiquidsInside` true)
          (elif (and (== (`self.FluidInsideID`) 4) (not (`self.bAreTwoLiquidsInside`)))
            (switch `int` FluidID
              (:`1`
                (bind _returnvalue_14 (`|GetDataTableRow` _datatable_13 _rowname_13)
                  (:`then`
                    (`NiagaraComponent.SetVariableLinearColor` (`self.Flow`) "Color" (`.Color_5_710DF73E405FA430BE76E1955AAA3F73` (break `/Game/EducationVR/Data/S_FluidColors` _returnvalue_14)))
                    (`NiagaraComponent.SetVariableMaterial` (`self.Fluid`) "Material" "/Game/LiquidMaterials_VFXPack/Materials/Liquids/MI_Liquid_Colorless_Brown.MI_Liquid_Colorless_Brown"))))
              (:`2`
                (bind _returnvalue_15 (`|GetDataTableRow` _datatable_15 _rowname_15)
                  (:`then`
                    (`NiagaraComponent.SetVariableLinearColor` (`self.Flow`) "Color" (`.Color_5_710DF73E405FA430BE76E1955AAA3F73` (break `/Game/EducationVR/Data/S_FluidColors` _returnvalue_15)))
                    (`NiagaraComponent.SetVariableMaterial` (`self.Fluid`) "Material" "/Game/LiquidMaterials_VFXPack/Materials/Liquids/MI_Liquid_Brown.MI_Liquid_Brown"))))
              (:`3`
                (bind _returnvalue_16 (`|GetDataTableRow` _datatable _rowname)
                  (:`then`
                    (`NiagaraComponent.SetVariableLinearColor` (`self.Flow`) "Color" (`.Color_5_710DF73E405FA430BE76E1955AAA3F73` (break `/Game/EducationVR/Data/S_FluidColors` _returnvalue_16)))
                    (`NiagaraComponent.SetVariableMaterial` (`self.Fluid`) "Material" "/Game/LiquidMaterials_VFXPack/Materials/Liquids/MI_Liquid_GreenishBrown.MI_Liquid_GreenishBrown"))))
              (:`4`
                (return)))
            (set `self.bAreTwoLiquidsInside` true)))))))

(fn `FillContainer`
  (bind _returnvalue (+ (`self.FluidLevel`) 0.01))
  (if (and (< (`self.FluidLevel`) 1.0) (`/Game/EducationVR/Blueprints/Chemistry/BP_FlaskParent.bIsPouring` (`self.Flask`)))
    (set `self.bIsLiquidInside` true)
    (`self.DetermineFluidColor` (`/Game/EducationVR/Blueprints/Chemistry/BP_FlaskParent.ID` (`self.Flask`)))
    (`NiagaraComponent.SetVariableFloat` (`self.Fluid`) "Fill" _returnvalue)
    (set `self.FluidLevel` _returnvalue)))

(fn `UserConstructionScript`)