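; BP_FlaskParent is a flask Blueprint, apparently a base class for EducationVR chemistry, that handles pouring liquid when tilted.
; Tick, throttled by a short Delay, compares the mesh up vector's Z to a rotation threshold and checks for liquid inside.
; When both conditions hold, it activates the Flow effect, sets IsPouring and replays audio on a timed guard; otherwise it stops all three.
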(event `self.ReceiveTick`
  (params (DeltaSeconds :type "Float (single-precision)"))
  (bind (_returnvalue_x _returnvalue_y _returnvalue_z) (`KismetMathLibrary.BreakVector` (`SceneComponent.GetUpVector` (`self.StaticMesh`))))
  (`KismetSystemLibrary.Delay` 0.1)
  (if (< _returnvalue_z (`self.RotationThreshold`))
    (if (`self.bIsLiquidInside`)
      (`ActorComponent.SetActive` (`self.Flow`) true false)
      (set `self.bIsPouring` true)
      (if (not (`self.bIsSoundPlaying`))
        (set `self.bIsSoundPlaying` true)
        (`AudioComponent.Play` (`self.Audio`) 0.0)
        (`KismetSystemLibrary.Delay` 3.8)
        (set `self.bIsSoundPlaying` false))
      (else
        (`ActorComponent.SetActive` (`self.Flow`) false false :!label _label)
        (set `self.bIsPouring` false)
        (set `self.bIsSoundPlaying` false)
        (`AudioComponent.Stop` (`self.Audio`))))
    (else
      (goto _label))))

(fn `UserConstructionScript`)