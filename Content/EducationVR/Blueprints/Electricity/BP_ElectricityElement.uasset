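; Grabbable electricity element for a VR education game that snaps into circuit slots when dropped.
; A drop within range of a slot, on an element tagged SlotElement, destroys any occupant, then locks the element static at the slot's drop point.
; Placing it also spawns a replacement at its respawn location, attaching both to the confirm button's current model manager.
; Otherwise, a still-grabbable element falls with physics.
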(event `self.GrabComponent.OnDropped`
  (bind _slotactor (`self.SlotActor`))
  (if (`self.bCanBeGrabbed`)
    (if (and (`self.bIsInSlotRange`) (`self.ActorHasTag` self "SlotElement") true)
      (set `self.bCanBeGrabbed` false)
      (`self.RecreateActor` self)
      (if (`/Game/EducationVR/Blueprints/Electricity/BP_Slot.bIsActorOnTop` (`self.SlotActor`))
        (`self.K2_DestroyActor` (`/Game/EducationVR/Blueprints/Electricity/BP_Slot.ActorOnTop` (`self.SlotActor`)))
        (set `/Game/EducationVR/Blueprints/Electricity/BP_Slot.bIsActorOnTop` false (`self.SlotActor`)))
      (set `/Game/EducationVR/Blueprints/Electricity/BP_Slot.ActorOnTop` self (`self.SlotActor`))
      (`SceneComponent.K2_SetWorldTransform` (`self.StaticMesh`) (`KismetMathLibrary.MakeTransform` (`SceneComponent.K2_GetComponentLocation` (`/Game/EducationVR/Blueprints/Electricity/BP_Slot.ActorDropPoint` (`self.SlotActor`)))) false false)
      (bind _returnvalue (`GameplayStatics.GetActorOfClass` "/Game/EducationVR/Blueprints/Electricity/BP_ButtonConfirm.BP_ButtonConfirm_C"))
      (`self.K2_AttachToActor` self (`/Game/EducationVR/Blueprints/Electricity/BP_ButtonConfirm.CurrentModelManager` _returnvalue) "None" "KeepWorld" "KeepWorld" "KeepWorld" true)
      (`SceneComponent.SetMobility` (`self.StaticMesh`) "Static")
      (set `/Game/EducationVR/Blueprints/Electricity/BP_Slot.ActorOnTop` self _slotactor)
      (set `self.bHasSlot` true)
      (set `/Game/EducationVR/Blueprints/Electricity/BP_Slot.bIsActorOnTop` true _slotactor)
      (else
        (`SceneComponent.SetMobility` (`self.StaticMesh`) "Movable")
        (`PrimitiveComponent.SetSimulatePhysics` (`self.StaticMesh`) true)))))

(fn `RecreateActor`
  (params (ActorToCreate :type "/Game/EducationVR/Blueprints/Electricity/BP_ElectricityElement Object Reference"))
  (bind _returnvalue (`|SpawnActorFromClass` (`GameplayStatics.GetObjectClass` ActorToCreate) (`KismetMathLibrary.MakeTransform` (`self.RespawnLocation`)) "Undefined" "MultiplyWithRoot" null null null null 0.0 3.0 9.0 (0.0 0.0 0.0) false true null))
  (bind _returnvalue_2 (`GameplayStatics.GetActorOfClass` "/Game/EducationVR/Blueprints/Electricity/BP_ButtonConfirm.BP_ButtonConfirm_C"))
  (`self.K2_AttachToActor` _returnvalue (`/Game/EducationVR/Blueprints/Electricity/BP_ButtonConfirm.CurrentModelManager` _returnvalue_2) "None" "KeepWorld" "KeepWorld" "KeepWorld" true)
  (set `/Game/EducationVR/Blueprints/Electricity/BP_ElectricityElement.RespawnLocation` (`self.RespawnLocation`) _returnvalue)
  (set `self.RequiredVoltage` (`self.RequiredVoltage`))
  (`SceneComponent.SetVisibility` (`/Game/EducationVR/Blueprints/Electricity/BP_ElectricityElement.StaticMesh` _returnvalue) true true)
  (set `/Game/VRTemplate/Blueprints/GrabComponent.GrabType` "NewEnumerator4" (`/Game/EducationVR/Blueprints/Electricity/BP_ElectricityElement.GrabComponent` _returnvalue)))

(fn `UserConstructionScript`)