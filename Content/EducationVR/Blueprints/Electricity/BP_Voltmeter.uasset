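; BP_Voltmeter is a voltmeter for the VR electricity education content that displays a voltage reading.
; A looping 0.1-second timer starts at BeginPlay, presumably driving SetVoltageTextAndMaterial.
; That function writes the voltage to a text render and switches a mesh material between green for positive and gray otherwise.
; It then copies voltage from the slot actor when slotted, so the display trails by one update.
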(event `self.ReceiveBeginPlay`
  (`KismetSystemLibrary.K2_SetTimerDelegate` (`|CreateDelegate` :!event `SetVoltageTextAndMaterial`) 0.1 true))

(fn `SetVoltageTextAndMaterial`
  (bind _staticmesh (`self.StaticMesh`))
  (`TextRenderComponent.K2_SetText` (`self.TextRender`) (`|FormatText` "{Voltage}V" (`self.Voltage`)))
  (if (> (`self.Voltage`) 0.0)
    (`PrimitiveComponent.SetMaterial` _staticmesh 2 "/Game/EducationVR/Materials/M_TGreen.M_TGreen")
    (else
      (`PrimitiveComponent.SetMaterial` _staticmesh 2 "/Game/EducationVR/Materials/M_TGray.M_TGray")))
  (if (`self.bHasSlot`)
    (set `self.Voltage` (`/Game/EducationVR/Blueprints/Electricity/BP_ElectricityElement.Voltage` (`self.SlotActor`)))))

(fn `UserConstructionScript`)