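; Light bulb for the VR electricity lessons that lights up when its voltage reaches the required level.
; BeginPlay starts a short looping timer, presumably to poll ChangeMaterialBasedOnVoltage.
; That function compares Voltage to RequiredVoltage, swaps the mesh between emissive and plain glass materials, and sets IsOn.
; It also starts the bulb sound once on switching on and stops it when off, if sound is allowed.
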(event `self.ReceiveBeginPlay`
  (`KismetSystemLibrary.K2_SetTimerDelegate` (`|CreateDelegate` :!event `ChangeMaterialBasedOnVoltage`) 0.1 true))

(fn `ChangeMaterialBasedOnVoltage`
  (bind _staticmesh (`self.StaticMesh`))
  (if (>= (`self.Voltage`) (`self.RequiredVoltage`))
    (`PrimitiveComponent.SetMaterial` _staticmesh 0 "/Game/EducationVR/Materials/M_GlassEmmisive2.M_GlassEmmisive2")
    (set `self.bIsOn` true)
    (if (not (`self.bIsSoundPlaying`))
      (set `self.bIsSoundPlaying` true)
      (if (`self.bCanSoundBePlayed`)
        (`AudioComponent.Play` (`self.SC_Lightbulb`) 0.0)))
    (else
      (`PrimitiveComponent.SetMaterial` _staticmesh 0 "/Game/EducationVR/Materials/M_Glass.M_Glass")
      (set `self.bIsOn` false)
      (set `self.bIsSoundPlaying` false)
      (if (`self.bCanSoundBePlayed`)
        (`AudioComponent.Stop` (`self.SC_Lightbulb`))))))

(fn `UserConstructionScript`)