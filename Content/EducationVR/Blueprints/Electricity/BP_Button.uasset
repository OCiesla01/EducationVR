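; BP_Button is a push button for the VR electricity education module, switching on only while pressed in a powered slot.
; Trigger begin overlap requires a valid SlotActor, HasSlot and positive Voltage, then sets IsOn and turns ButtonMain green.
; End overlap needs only HasSlot to clear IsOn and turn it red.
; Both transitions play a click sound at the mesh when CanSoundBePlayed allows.
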(event `self.ReceiveBeginPlay`)

(event `self.Trigger.OnComponentBeginOverlap`
  (params (OverlappedComponent :type "PrimitiveComponent Object Reference") (OtherActor :type "Actor Object Reference") (OtherComp :type "PrimitiveComponent Object Reference") (OtherBodyIndex :type Integer) (bFromSweep :type Boolean) (SweepResult :type "HitResult Structure (by ref)"))
  (bind _slotactor (`self.SlotActor`)
    (:`then`
      (if (and (`self.bHasSlot`) (> (`/Game/EducationVR/Blueprints/Electricity/BP_ElectricityElement.Voltage` _slotactor) 0.0))
        (set `self.bIsOn` true)
        (`PrimitiveComponent.SetMaterial` (`self.ButtonMain`) 0 "/Game/EducationVR/Materials/M_TGreen.M_TGreen")
        (if (`self.bCanSoundBePlayed`)
          (`GameplayStatics.PlaySoundAtLocation` "/Game/EducationVR/Audio/Electricity/button_on.button_on" (`SceneComponent.K2_GetComponentLocation` (`self.StaticMesh`)) (struct) 1.0 1.0 0.0 null null null null))))
    (:`else`)))

(event `self.Trigger.OnComponentEndOverlap`
  (params (OverlappedComponent :type "PrimitiveComponent Object Reference") (OtherActor :type "Actor Object Reference") (OtherComp :type "PrimitiveComponent Object Reference") (OtherBodyIndex :type Integer))
  (if (`self.bHasSlot`)
    (set `self.bIsOn` false)
    (`PrimitiveComponent.SetMaterial` (`self.ButtonMain`) 0 "/Game/EducationVR/Materials/M_TRed.M_TRed")
    (if (`self.bCanSoundBePlayed`)
      (`GameplayStatics.PlaySoundAtLocation` "/Game/EducationVR/Audio/Electricity/button_off.button_off" (`SceneComponent.K2_GetComponentLocation` (`self.StaticMesh`)) (struct) 1.0 1.0 0.0 null null null null))))

(fn `UserConstructionScript`)