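; BP_Diode is an electricity component in EducationVR that shows whether its voltage lies within a working range.
; CheckVoltage compares Voltage against required and maximum limits, sets IsOn, and swaps a mesh material between emissive and plain glass.
; BeginPlay starts a short looping timer, though the graph does not name the function it calls.
; Nothing in this Blueprint sets Voltage.
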(event `self.ReceiveBeginPlay`
  (`KismetSystemLibrary.K2_SetTimerDelegate` (`|CreateDelegate` :!event `CheckVoltage`) 0.1 true))

(fn `CheckVoltage`
  (bind _staticmesh (`self.StaticMesh`))
  (if (and (>= (`self.Voltage`) (`self.RequiredVoltage`)) (<= (`self.Voltage`) (`self.MaxVoltage`)))
    (`PrimitiveComponent.SetMaterial` _staticmesh 1 "/Game/EducationVR/Materials/M_GlassEmmisive.M_GlassEmmisive")
    (set `self.bIsOn` true)
    (else
      (`PrimitiveComponent.SetMaterial` _staticmesh 1 "/Game/EducationVR/Materials/M_Glass.M_Glass")
      (set `self.bIsOn` false))))

(fn `UserConstructionScript`)