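; Battery actor for a VR electricity lesson, with a main switch and three cable exits operated by overlap triggers.
; Exit buttons work only when switched on and connected, toggling colour and splitting total voltage equally among active exits' cables.
; Timers debounce each button.
; Switching off resets all exits and cable voltages, but this reset and the switch's timeline rotation run only when CanSoundBePlayed is true.
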(event `self.TriggerLeft.OnComponentBeginOverlap`
  (params (OverlappedComponent :type "PrimitiveComponent Object Reference") (OtherActor :type "Actor Object Reference") (OtherComp :type "PrimitiveComponent Object Reference") (OtherBodyIndex :type Integer) (bFromSweep :type Boolean) (SweepResult :type "HitResult Structure (by ref)"))
  (bind _buttonleft (`self.ButtonLeft`))
  (bind _exitson (`self.ExitsOn`))
  (bind _returnvalue (`SceneComponent.K2_GetComponentLocation` (`self.StaticMesh`)))
  (if (`self.bCanBeUsed`)
    (if (`self.bIsOn`)
      (if (`self.bIsLeftConnected`)
        (if (`self.bCanPressLeftButton`)
          (set `self.bCanPressLeftButton` false)
          (`KismetSystemLibrary.K2_SetTimerDelegate` (`|CreateDelegate` :!event `ResetLeftButton`) 0.5)
          (if (`self.bIsLeftActive`)
            (set `self.bIsLeftActive` false)
            (`PrimitiveComponent.SetMaterial` _buttonleft 0 "/Game/EducationVR/Materials/M_TRed.M_TRed")
            (`/Engine/EditorBlueprintResources/StandardMacros.DecrementInt` _exitson
              (:`  `
                (`self.SetVoltagePerExit`)
                (`self.SetCablesVoltage`)
                (if (`self.bCanSoundBePlayed`)
                  (`GameplayStatics.PlaySoundAtLocation` "/Game/EducationVR/Audio/Electricity/button_off.button_off" _returnvalue (struct) 1.0 1.0 0.0 null null null null))))
            (else
              (set `self.bIsLeftActive` true)
              (`PrimitiveComponent.SetMaterial` _buttonleft 0 "/Game/EducationVR/Materials/M_TGreen.M_TGreen")
              (`/Engine/EditorBlueprintResources/StandardMacros.IncrementInt` _exitson
                (:`  `
                  (`self.SetVoltagePerExit`)
                  (`self.SetCablesVoltage`)
                  (if (`self.bCanSoundBePlayed`)
                    (`GameplayStatics.PlaySoundAtLocation` "/Game/EducationVR/Audio/Electricity/button_on.button_on" _returnvalue (struct) 1.0 1.0 0.0 null null null null)))))))))))

(event `self.TriggerMid.OnComponentBeginOverlap`
  (params (OverlappedComponent :type "PrimitiveComponent Object Reference") (OtherActor :type "Actor Object Reference") (OtherComp :type "PrimitiveComponent Object Reference") (OtherBodyIndex :type Integer) (bFromSweep :type Boolean) (SweepResult :type "HitResult Structure (by ref)"))
  (bind _buttonmid (`self.ButtonMid`))
  (bind _exitson (`self.ExitsOn`))
  (bind _returnvalue (`SceneComponent.K2_GetComponentLocation` (`self.StaticMesh`)))
  (if (`self.bCanBeUsed`)
    (if (`self.bIsOn`)
      (if (`self.bIsMidConnected`)
        (if (`self.bCanPressMiddleButton`)
          (set `self.bCanPressMiddleButton` false)
          (`KismetSystemLibrary.K2_SetTimerDelegate` (`|CreateDelegate` :!event `ResetMidButton`) 0.5)
          (if (`self.bIsMidActive`)
            (set `self.bIsMidActive` false)
            (`PrimitiveComponent.SetMaterial` _buttonmid 0 "/Game/EducationVR/Materials/M_TRed.M_TRed")
            (`/Engine/EditorBlueprintResources/StandardMacros.DecrementInt` _exitson
              (:`  `
                (`self.SetVoltagePerExit`)
                (`self.SetCablesVoltage`)
                (if (`self.bCanSoundBePlayed`)
                  (`GameplayStatics.PlaySoundAtLocation` "/Game/EducationVR/Audio/Electricity/button_off.button_off" _returnvalue (struct) 1.0 1.0 0.0 null null null null))))
            (else
              (set `self.bIsMidActive` true)
              (`PrimitiveComponent.SetMaterial` _buttonmid 0 "/Game/EducationVR/Materials/M_TGreen.M_TGreen")
              (`/Engine/EditorBlueprintResources/StandardMacros.IncrementInt` _exitson
                (:`  `
                  (`self.SetVoltagePerExit`)
                  (`self.SetCablesVoltage`)
                  (if (`self.bCanSoundBePlayed`)
                    (`GameplayStatics.PlaySoundAtLocation` "/Game/EducationVR/Audio/Electricity/button_on.button_on" _returnvalue (struct) 1.0 1.0 0.0 null null null null)))))))))))

(event `self.TriggerRight.OnComponentBeginOverlap`
  (params (OverlappedComponent :type "PrimitiveComponent Object Reference") (OtherActor :type "Actor Object Reference") (OtherComp :type "PrimitiveComponent Object Reference") (OtherBodyIndex :type Integer) (bFromSweep :type Boolean) (SweepResult :type "HitResult Structure (by ref)"))
  (bind _buttonright (`self.ButtonRight`))
  (bind _exitson (`self.ExitsOn`))
  (bind _returnvalue (`SceneComponent.K2_GetComponentLocation` (`self.StaticMesh`)))
  (if (`self.bCanBeUsed`)
    (if (`self.bIsOn`)
      (if (`self.bIsRightConnected`)
        (if (`self.bCanPressRightButton`)
          (set `self.bCanPressRightButton` false)
          (`KismetSystemLibrary.K2_SetTimerDelegate` (`|CreateDelegate` :!event `ResetRightButton`) 0.5)
          (if (`self.bIsRightActive`)
            (set `self.bIsRightActive` false)
            (`PrimitiveComponent.SetMaterial` _buttonright 0 "/Game/EducationVR/Materials/M_TRed.M_TRed")
            (`/Engine/EditorBlueprintResources/StandardMacros.DecrementInt` _exitson
              (:`  `
                (`self.SetVoltagePerExit`)
                (`self.SetCablesVoltage`)
                (if (`self.bCanSoundBePlayed`)
                  (`GameplayStatics.PlaySoundAtLocation` "/Game/EducationVR/Audio/Electricity/button_off.button_off" _returnvalue (struct) 1.0 1.0 0.0 null null null null))))
            (else
              (set `self.bIsRightActive` true)
              (`PrimitiveComponent.SetMaterial` _buttonright 0 "/Game/EducationVR/Materials/M_TGreen.M_TGreen")
              (`/Engine/EditorBlueprintResources/StandardMacros.IncrementInt` _exitson
                (:`  `
                  (`self.SetVoltagePerExit`)
                  (`self.SetCablesVoltage`)
                  (if (`self.bCanSoundBePlayed`)
                    (`GameplayStatics.PlaySoundAtLocation` "/Game/EducationVR/Audio/Electricity/button_on.button_on" _returnvalue (struct) 1.0 1.0 0.0 null null null null)))))))))))

(event `self.TriggerSwitch.OnComponentBeginOverlap`
  (params (OverlappedComponent :type "PrimitiveComponent Object Reference") (OtherActor :type "Actor Object Reference") (OtherComp :type "PrimitiveComponent Object Reference") (OtherBodyIndex :type Integer) (bFromSweep :type Boolean) (SweepResult :type "HitResult Structure (by ref)"))
  (bind _switchbutton (`self.SwitchButton`))
  (bind _bcansoundbeplayed (`self.bCanSoundBePlayed`))
  (bind _returnvalue (`SceneComponent.K2_GetComponentLocation` (`self.StaticMesh`)))
  (if (`self.bCanBeUsed`)
    (if (`self.bIsOn`)
      (if (`self.bCanPressSwitchButton`)
        (set `self.bCanPressSwitchButton` false)
        (`KismetSystemLibrary.K2_SetTimerDelegate` (`|CreateDelegate` :!event `ResetSwitchButton`) 0.5)
        (set `self.bIsOn` false)
        (`PrimitiveComponent.SetMaterial` _switchbutton 0 "/Game/EducationVR/Materials/M_TRed.M_TRed")
        (if _bcansoundbeplayed
          (`GameplayStatics.PlaySoundAtLocation` "/Game/EducationVR/Audio/Electricity/switch_off.switch_off" _returnvalue (struct) 1.0 1.0 0.0 null null null null)
          (`self.DeactivateAll`)
          (bind (_direction _alpha) (`Timeline|T_ButtonRotation` :!label _label)
            (:`Update`
              (`SceneComponent.K2_SetWorldRotation` (`self.SwitchButton`) (`KismetMathLibrary.MakeRotator` (`KismetMathLibrary.Lerp` -12.0 12.0 _alpha)) false false)))))
      (elif (`self.bCanPressSwitchButton`)
        (set `self.bCanPressSwitchButton` false)
        (`KismetSystemLibrary.K2_SetTimerDelegate` (`|CreateDelegate` :!event `ResetSwitchButton`) 0.5)
        (set `self.bIsOn` true)
        (`PrimitiveComponent.SetMaterial` _switchbutton 0 "/Game/EducationVR/Materials/M_TGreen.M_TGreen")
        (if _bcansoundbeplayed
          (`GameplayStatics.PlaySoundAtLocation` "/Game/EducationVR/Audio/Electricity/switch_on.switch_on" _returnvalue (struct) 1.0 1.0 0.0 null null null null)
          (goto _label :!via `Reverse`))))))

(event `ResetRightButton`
  (set `self.bCanPressRightButton` true))

(event `ResetMidButton`
  (set `self.bCanPressMiddleButton` true))

(event `ResetLeftButton`
  (set `self.bCanPressLeftButton` true))

(event `ResetSwitchButton`
  (set `self.bCanPressSwitchButton` true))

(fn `DeactivateAll`
  (set `self.bIsLeftActive` false)
  (set `self.bIsRightActive` false)
  (set `self.bIsMidActive` false)
  (`PrimitiveComponent.SetMaterial` (`self.ButtonLeft`) 0 "/Game/EducationVR/Materials/M_TRed.M_TRed")
  (`PrimitiveComponent.SetMaterial` (`self.ButtonMid`) 0 "/Game/EducationVR/Materials/M_TRed.M_TRed")
  (`PrimitiveComponent.SetMaterial` (`self.ButtonRight`) 0 "/Game/EducationVR/Materials/M_TRed.M_TRed")
  (set `self.ExitsOn` 0)
  (set `self.VoltagePerExit` 0.0)
  (bind _cableleft (`self.CableLeft`)
    (:`then`
      (set `/Game/EducationVR/Blueprints/Electricity/BP_ElectricityElement.Voltage` 0.0 _cableleft))
    (:`else`
      _))
  (bind _cablemid (`self.CableMid`)
    (:`then`
      (set `/Game/EducationVR/Blueprints/Electricity/BP_ElectricityElement.Voltage` 0.0 _cablemid))
    (:`else`
      _))
  (bind _cableright (`self.CableRight`)
    (:`then`
      (set `/Game/EducationVR/Blueprints/Electricity/BP_ElectricityElement.Voltage` 0.0 _cableright))
    (:`else`)))

(fn `SetCablesVoltage`
  (`|ExecutionSequence`
    (:`then_0`
      (if (`self.bIsLeftConnected`)
        (if (`self.bIsLeftActive`)
          (set `/Game/EducationVR/Blueprints/Electricity/BP_ElectricityElement.Voltage` (`self.VoltagePerExit`) (`self.CableLeft`))
          (else
            (set `/Game/EducationVR/Blueprints/Electricity/BP_ElectricityElement.Voltage` 0.0 (`self.CableLeft`))))))
    (:`then_1`
      (if (`self.bIsMidConnected`)
        (if (`self.bIsMidActive`)
          (set `/Game/EducationVR/Blueprints/Electricity/BP_ElectricityElement.Voltage` (`self.VoltagePerExit`) (`self.CableMid`))
          (else
            (set `/Game/EducationVR/Blueprints/Electricity/BP_ElectricityElement.Voltage` 0.0 (`self.CableMid`))))))
    (:`then_2`
      (if (`self.bIsRightConnected`)
        (if (`self.bIsRightActive`)
          (set `/Game/EducationVR/Blueprints/Electricity/BP_ElectricityElement.Voltage` (`self.VoltagePerExit`) (`self.CableRight`))
          (else
            (set `/Game/EducationVR/Blueprints/Electricity/BP_ElectricityElement.Voltage` 0.0 (`self.CableRight`))))))))

(fn `SetVoltagePerExit`
  (returns (Voltage :type "Float (double-precision)"))
  (bind _output_get (set `self.VoltagePerExit` (/ (`self.TotalVoltage`) (`self.ExitsOn`))))
  (return _output_get))

(fn `UserConstructionScript`)