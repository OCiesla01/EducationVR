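; VR confirm button for the electricity lesson that advances from one circuit model to the next.
; Overlapping its trigger starts a three-second timer; if still pressed when NextModel runs, it hides the current model and shows the next after a short delay.
; Models are matched by number in an array, toggling attached elements, text, slots and battery use.
; Showing a model also spawns its grabbable objects, attached to that model's manager.
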(event `self.Trigger.OnComponentBeginOverlap`
  (params (OverlappedComponent :type "PrimitiveComponent Object Reference") (OtherActor :type "Actor Object Reference") (OtherComp :type "PrimitiveComponent Object Reference") (OtherBodyIndex :type Integer) (bFromSweep :type Boolean) (SweepResult :type "HitResult Structure (by ref)"))
  (set `self.bIsPressed` true)
  (`KismetSystemLibrary.K2_SetTimerDelegate` (`|CreateDelegate` :!event `NextModel`) 3.0))

(event `self.Trigger.OnComponentEndOverlap`
  (params (OverlappedComponent :type "PrimitiveComponent Object Reference") (OtherActor :type "Actor Object Reference") (OtherComp :type "PrimitiveComponent Object Reference") (OtherBodyIndex :type Integer))
  (set `self.bIsPressed` false))

(event `NextModel`
  (bind _currentmodel (`self.CurrentModel`))
  (if (`self.bIsPressed`)
    (`self.HideModel` (`self.CurrentModel`))
    (`/Engine/EditorBlueprintResources/StandardMacros.IncrementInt` _currentmodel
      (:`  `
        (`KismetSystemLibrary.Delay` 1.0)
        (`self.ShowModel` _currentmodel)))))

(fn `CreateObjects`
  (for _array_element (`/Game/EducationVR/Blueprints/Electricity/BP_ModelManager.ObjectsToCreate` (`self.CurrentModelManager`))
    (bind _output_get (set `/Game/EducationVR/Blueprints/Electricity/BP_ElectricityElement.RespawnLocation` (`/Game/EducationVR/Blueprints/Electricity/BP_ElectricityElement.RespawnLocation` _array_element) _array_element))
    (bind _returnvalue (`|SpawnActorFromClass` (`GameplayStatics.GetObjectClass` _array_element) (`KismetMathLibrary.MakeTransform` _output_get) "Undefined" "MultiplyWithRoot" null null null null 0.0 (`/Game/EducationVR/Blueprints/Electricity/BP_ElectricityElement.RequiredVoltage` _array_element) (`/Game/EducationVR/Blueprints/Electricity/BP_ElectricityElement.MaxVoltage` _array_element) _output_get false true null))
    (`self.K2_AttachToActor` _returnvalue (`self.CurrentModelManager`) "None" "KeepWorld" "KeepWorld" "KeepWorld" true)
    (set `/Game/VRTemplate/Blueprints/GrabComponent.GrabType` "NewEnumerator4" (`/Game/EducationVR/Blueprints/Electricity/BP_ElectricityElement.GrabComponent` _returnvalue))
    (`SceneComponent.SetVisibility` (`/Game/EducationVR/Blueprints/Electricity/BP_ElectricityElement.StaticMesh` _returnvalue) true true)))

(fn `HideModel`
  (params (CurrentModel :type Integer))
  (if (> (`self.CurrentModel`) 0)
    (for _array_element (`self.ModelsArr`)
      (if (== (`/Game/EducationVR/Blueprints/Electricity/BP_ModelManager.ModelNumber` _array_element) CurrentModel)
        (for _array_element_2 (`self.GetAttachedActors` _array_element true false)
          (bind _asbp_electricity_element (cast `/Game/EducationVR/Blueprints/Electricity/BP_ElectricityElement` _array_element_2))
          (`SceneComponent.SetVisibility` (`/Game/EducationVR/Blueprints/Electricity/BP_ElectricityElement.StaticMesh` _asbp_electricity_element) false true)
          (set `/Game/EducationVR/Blueprints/Electricity/BP_ElectricityElement.bCanSoundBePlayed` false _asbp_electricity_element)
          (bind _asbp_slot (cast `/Game/EducationVR/Blueprints/Electricity/BP_Slot` _asbp_electricity_element))
          (set `/Game/EducationVR/Blueprints/Electricity/BP_ElectricityElement.bIsOn` false _asbp_slot))
        (`SceneComponent.SetVisibility` (`TextRenderActor.TextRender` (`/Game/EducationVR/Blueprints/Electricity/BP_ModelManager.Text` _array_element)) false false)
        (set `/Game/EducationVR/Blueprints/Electricity/BP_Battery.bCanBeUsed` false (`/Game/EducationVR/Blueprints/Electricity/BP_ModelManager.Battery` (`self.CurrentModelManager`)))))))

(fn `ShowModel`
  (params (CurrentModel :type Integer))
  (for _array_element (`self.ModelsArr`)
    (if (== (`/Game/EducationVR/Blueprints/Electricity/BP_ModelManager.ModelNumber` _array_element) CurrentModel)
      (set `self.CurrentModelManager` _array_element)
      (for _array_element_2 (`self.GetAttachedActors` _array_element true false)
        (bind _asbp_electricity_element (cast `/Game/EducationVR/Blueprints/Electricity/BP_ElectricityElement` _array_element_2))
        (`SceneComponent.SetVisibility` (`/Game/EducationVR/Blueprints/Electricity/BP_ElectricityElement.StaticMesh` _asbp_electricity_element) true true)
        (bind _asbp_slot (cast `/Game/EducationVR/Blueprints/Electricity/BP_Slot` _asbp_electricity_element))
        (set `/Game/EducationVR/Blueprints/Electricity/BP_ElectricityElement.bIsOn` true _asbp_slot))
      (`SceneComponent.SetVisibility` (`TextRenderActor.TextRender` (`/Game/EducationVR/Blueprints/Electricity/BP_ModelManager.Text` _array_element)) true false)
      (set `/Game/EducationVR/Blueprints/Electricity/BP_Battery.bCanBeUsed` true (`/Game/EducationVR/Blueprints/Electricity/BP_ModelManager.Battery` (`self.CurrentModelManager`)))
      (`self.CreateObjects`))))

(fn `UserConstructionScript`)