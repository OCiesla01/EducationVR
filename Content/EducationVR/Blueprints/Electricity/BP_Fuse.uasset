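; BP_Fuse is an electricity module for the VR education game that breaks when its voltage reaches a limit.
; CalculateVoltage sums three entry voltages and, on first reaching MaxVoltage, marks the fuse broken, plays an explosion sound at the mesh and calls CallModuleEnd.
; BeginPlay starts a looping 0.1-second timer, though the event it drives is not shown.
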(event `self.ReceiveBeginPlay`
  (`KismetSystemLibrary.K2_SetTimerDelegate` (`|CreateDelegate` :!event `CalculateVoltage`) 0.1 true))

(fn `CalculateVoltage`
  (bind _output_get (set `self.Voltage` (+ (`self.Entry1Voltage`) (`self.Entry2Voltage`) (`self.Entry3Voltage`))))
  (if (and (>= _output_get (`self.MaxVoltage`)) (not (`self.bIsBroken`)))
    (set `self.bIsBroken` true)
    (`GameplayStatics.PlaySoundAtLocation` "/Game/EducationVR/Audio/Electricity/fuse_explosion.fuse_explosion" (`SceneComponent.K2_GetComponentLocation` (`self.StaticMesh`)) (struct) 1.0 1.0 0.0 null null null null)
    (`self.ModuleEnd`)))

(fn `UserConstructionScript`)