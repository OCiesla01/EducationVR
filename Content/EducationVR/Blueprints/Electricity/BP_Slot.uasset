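; BP_Slot is a socket in the VR education electricity exercise that holds electricity elements and relays voltage through them.
; While on, its trigger tells overlapping elements they are in range and which slot they are near, clearing this on exit.
; Its functions copy voltage to the element on top and to ActorEnd, with gates switching it and resistors halving it.
; BeginPlay starts two fast looping timers, presumably to poll this propagation.
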(event `self.ReceiveBeginPlay`
  (`KismetSystemLibrary.K2_SetTimerDelegate` (`|CreateDelegate` :!event `PassVoltageIfAvailable`) 0.1 true)
  (`KismetSystemLibrary.K2_SetTimerDelegate` (`|CreateDelegate` :!event `PassVoltageToActorOnTop`) 0.1 true))

(event `self.Trigger.OnComponentBeginOverlap`
  (params (OverlappedComponent :type "PrimitiveComponent Object Reference") (OtherActor :type "Actor Object Reference") (OtherComp :type "PrimitiveComponent Object Reference") (OtherBodyIndex :type Integer) (bFromSweep :type Boolean) (SweepResult :type "HitResult Structure (by ref)"))
  (if (`self.bIsOn`)
    (bind _asbp_electricity_element (cast `/Game/EducationVR/Blueprints/Electricity/BP_ElectricityElement` OtherActor))
    (set `/Game/EducationVR/Blueprints/Electricity/BP_ElectricityElement.SlotActor` self _asbp_electricity_element)
    (set `/Game/EducationVR/Blueprints/Electricity/BP_ElectricityElement.bIsInSlotRange` true _asbp_electricity_element)))

(event `self.Trigger.OnComponentEndOverlap`
  (params (OverlappedComponent :type "PrimitiveComponent Object Reference") (OtherActor :type "Actor Object Reference") (OtherComp :type "PrimitiveComponent Object Reference") (OtherBodyIndex :type Integer))
  (if (`self.bIsOn`)
    (bind _asbp_electricity_element (cast `/Game/EducationVR/Blueprints/Electricity/BP_ElectricityElement` OtherActor))
    (set `/Game/EducationVR/Blueprints/Electricity/BP_ElectricityElement.SlotActor` null _asbp_electricity_element)
    (set `/Game/EducationVR/Blueprints/Electricity/BP_ElectricityElement.bIsInSlotRange` false _asbp_electricity_element)))

(fn `PassVoltageIfAvailable`
  (bind _actorend (`self.ActorEnd`))
  (if (`self.bIsActorOnTop`)
    (if (`self.ActorHasTag` (`self.ActorOnTop`) "VoltageGate")
      (if (`/Game/EducationVR/Blueprints/Electricity/BP_ElectricityElement.bIsOn` (`self.ActorOnTop`))
        (set `/Game/EducationVR/Blueprints/Electricity/BP_ElectricityElement.Voltage` (`self.Voltage`) _actorend)
        (else
          (set `/Game/EducationVR/Blueprints/Electricity/BP_ElectricityElement.Voltage` 0.0 _actorend)))
      (elif (`self.ActorHasTag` (`self.ActorOnTop`) "Resistor")
        (set `/Game/EducationVR/Blueprints/Electricity/BP_ElectricityElement.Voltage` (/ (`self.Voltage`) 2.0) (`self.ActorEnd`))
        (else
          (set `/Game/EducationVR/Blueprints/Electricity/BP_ElectricityElement.Voltage` (`self.Voltage`) (`self.ActorEnd`)))))
    (else
      (set `/Game/EducationVR/Blueprints/Electricity/BP_ElectricityElement.Voltage` 0.0 (`self.ActorEnd`)))))

(fn `PassVoltageToActorOnTop`
  (if (`self.bIsActorOnTop`)
    (set `/Game/EducationVR/Blueprints/Electricity/BP_ElectricityElement.Voltage` (`self.Voltage`) (`self.ActorOnTop`))))

(fn `UserConstructionScript`)