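; BP_Switch is an electricity switch for the VR education game, toggled whenever something begins overlapping its Trigger component.
; It always allows switching off, but switches on only if a valid SlotActor reports Voltage above zero.
; Each change swaps the button material between red and green and optionally plays a sound at the mesh.
; A CanPressButton flag with a short timer debounces presses, including failed switch-on attempts.
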(event `self.Trigger.OnComponentBeginOverlap`
  (params (OverlappedComponent :type "PrimitiveComponent Object Reference") (OtherActor :type "Actor Object Reference") (OtherComp :type "PrimitiveComponent Object Reference") (OtherBodyIndex :type Integer) (bFromSweep :type Boolean) (SweepResult :type "HitResult Structure (by ref)"))
  (if (`self.bIsOn`)
    (if (`self.bCanPressButton`)
      (set `self.bCanPressButton` false)
      (`KismetSystemLibrary.K2_SetTimerDelegate` (`|CreateDelegate` :!event `ResetButton`) 0.5)
      (set `self.bIsOn` false)
      (`PrimitiveComponent.SetMaterial` (`self.SwitchButton`) 0 "/Game/EducationVR/Materials/M_TRed.M_TRed")
      (if (`self.bCanSoundBePlayed`)
        (`GameplayStatics.PlaySoundAtLocation` "/Game/EducationVR/Audio/Electricity/switch_off.switch_off" (`SceneComponent.K2_GetComponentLocation` (`self.StaticMesh`)) (struct) 1.0 1.0 0.0 null null null null)))
    (elif (`self.bCanPressButton`)
      (set `self.bCanPressButton` false)
      (`KismetSystemLibrary.K2_SetTimerDelegate` (`|CreateDelegate` :!event `ResetButton`) 0.5)
      (bind _slotactor (`self.SlotActor`)
        (:`then`
          (if (> (`/Game/EducationVR/Blueprints/Electricity/BP_ElectricityElement.Voltage` _slotactor) 0.0)
            (set `self.bIsOn` true)
            (`PrimitiveComponent.SetMaterial` (`self.SwitchButton`) 0 "/Game/EducationVR/Materials/M_TGreen.M_TGreen")
            (if (`self.bCanSoundBePlayed`)
              (`GameplayStatics.PlaySoundAtLocation` "/Game/EducationVR/Audio/Electricity/switch_on.switch_on" (`SceneComponent.K2_GetComponentLocation` (`self.StaticMesh`)) (struct) 1.0 1.0 0.0 null null null null))))
        (:`else`)))))

(event `ResetButton`
  (set `self.bCanPressButton` true))

(fn `UserConstructionScript`)