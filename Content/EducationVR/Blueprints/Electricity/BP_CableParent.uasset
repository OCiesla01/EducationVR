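; BP_CableParent is the base cable in the EducationVR electricity setup, passing its Voltage to the actor at its end.
; BeginPlay starts a fast looping timer, though the event it calls is not shown.
; GiveVoltage writes directly to the end actor's Voltage or, for fuse cables, casts it to BP_Fuse and sets one of three entry voltages chosen by FuseEntry.
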(event `self.ReceiveBeginPlay`
  (`KismetSystemLibrary.K2_SetTimerDelegate` (`|CreateDelegate` :!event `GiveVoltage`) 0.1 true))

(fn `GiveVoltage`
  (bind _voltage (`self.Voltage`))
  (if (`self.bIsFuseCable`)
    (bind _asbp_fuse (cast `/Game/EducationVR/Blueprints/Electricity/BP_Fuse` (`self.ActorEnd`)))
    (switch `int` (`self.FuseEntry`)
      (:`1`
        (set `/Game/EducationVR/Blueprints/Electricity/BP_Fuse.Entry1Voltage` _voltage _asbp_fuse))
      (:`2`
        (set `/Game/EducationVR/Blueprints/Electricity/BP_Fuse.Entry2Voltage` _voltage _asbp_fuse))
      (:`3`
        (set `/Game/EducationVR/Blueprints/Electricity/BP_Fuse.Entry3Voltage` _voltage _asbp_fuse)))
    (else
      (set `/Game/EducationVR/Blueprints/Electricity/BP_ElectricityElement.Voltage` (`self.Voltage`) (`self.ActorEnd`)))))

(fn `UserConstructionScript`)