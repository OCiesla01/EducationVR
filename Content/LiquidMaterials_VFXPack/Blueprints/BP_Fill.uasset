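; BP_Fill is a demo actor for the liquid materials VFX pack that cycles a liquid's fill level and displays the value.
; A delayed self-calling event raises Fill every few seconds, wraps it back to a low level, and pushes it to the Liquid component's User.Fill parameter and a text label.
; Tick continuously spins the static mesh and turns the label toward the player camera.
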(event `Again`
  (bind _fill (`self.Fill`))
  (`KismetSystemLibrary.Delay` 4.0 :!label _label)
  (bind _output_get (set `self.Fill` (+ (`self.Fill`) 0.2)))
  (if (> _output_get 1.1)
    (set `self.Fill` 0.2))
  (`FXSystemComponent.SetFloatParameter` (`self.Liquid`) "User.Fill" _fill)
  (`TextRenderComponent.K2_SetText` (`self.TextRender`) (`KismetTextLibrary.Conv_StringToText` (`KismetStringLibrary.Concat_StrStr` "Fill : " (`KismetStringLibrary.Conv_DoubleToString` _fill))))
  (`self.Again`))

(event `self.ReceiveBeginPlay`
  (bind _fill (`self.Fill`))
  (`FXSystemComponent.SetFloatParameter` (`self.Liquid`) "User.Fill" _fill)
  (`TextRenderComponent.K2_SetText` (`self.TextRender`) (`KismetTextLibrary.Conv_StringToText` (`KismetStringLibrary.Concat_StrStr` "Fill : " (`KismetStringLibrary.Conv_DoubleToString` _fill))))
  (goto _label))

(event `self.ReceiveTick`
  (params (DeltaSeconds :type "Float (single-precision)"))
  (`SceneComponent.K2_AddLocalRotation` (`self.StaticMesh`) (struct :`Pitch` 0.6 :`Yaw` 0.3 :`Roll` 1.0) false false)
  (`SceneComponent.K2_SetWorldRotation` (`self.TextRender`) (`KismetMathLibrary.MakeRotFromX` (- (`SceneComponent.K2_GetComponentLocation` (`PlayerCameraManager.TransformComponent` (`GameplayStatics.GetPlayerCameraManager` 0))) (`SceneComponent.K2_GetComponentLocation` (`self.TextRender`)))) false false))

(fn `UserConstructionScript`)